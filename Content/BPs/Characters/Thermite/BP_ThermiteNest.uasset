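; BP_ThermiteNest is a spawner that maintains a population of BP_Thermite characters in the game.
; From BeginPlay, it loops through a random delay and a spawn at its Cone component, repeating while the tracked array is below the maximum.
; Each thermite receives a reference to the nest.
; OnThermiteDied removes the dead one from the array and re-enters the respawn loop, which always spawns once before checking the cap.
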(event Custom|OnThermiteDied
  (params (WhoDied :type BP%20Thermite%20Object%20Reference))
  (Utilities|Array|RemoveItem (Variables|Default|GetSpawnedThermites) WhoDied)
  (CallFunction|RespawnThermite))

(event Custom|RespawnThermite
  (Utilities|FlowControl|Delay (Math|Random|RandomFloatinRange (Variables|Default|GetRespawnTimeMin) (Variables|Default|GetRespawnTimeMax)) :!label _label)
  (bind _returnvalue (Game|SpawnActorfromClass "/Game/BPs/Characters/Thermite/BP_Thermite.BP_Thermite_C" (Math|Transform|MakeTransform (Transformation|GetWorldLocation (Variables|Default|GetCone)) "0, 0, 0" "1.000000,1.000000,1.000000") "AdjustIfPossibleButAlwaysSpawn" "MultiplyWithRoot" 0 self 0))
  (Utilities|Array|Add (Variables|Default|GetSpawnedThermites) _returnvalue)
  (if (< (Utilities|Array|Length (Variables|Default|GetSpawnedThermites)) (Variables|Default|GetMaxThermiteNumber))
    (goto _label)))

(event EventBeginPlay
  (CallFunction|RespawnThermite))

(fn ConstructionScript)