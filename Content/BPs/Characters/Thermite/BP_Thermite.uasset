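; Thermite character Blueprint that belongs to a Nest and can be possessed.
; On death it notifies the Nest, stops its capsule blocking pawns and swaps its mesh to a red debug material.
; On possession it restores pawn blocking and sets the TargetActor blackboard key to empty for every thermite following the Nest.
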(event EventBeginPlay
  (|CallParentFunction) ; This node is disabled and will not be called.\nDrag off pins to build functionality.
)

(event Collision|EventActorBeginOverlap
  (params (OtherActor :type Actor%20Object%20Reference)))

(event EventTick
  (params (DeltaSeconds :type Float%20%28single-precision%29)))

(event EventOnDie
  (|CallParentFunction)
  (Default|OnThermiteDied (Variables|Default|GetNest))
  (Collision|SetCollisionResponsetoChannel (Variables|Default|GetCapsuleComponent) "ECC_Pawn" "ECR_Ignore")
  ;[1 0 0] FOR DEBUG
  (Rendering|Material|SetMaterial (Variables|Default|GetThermite_SM) 0 "/AnimationSharing/AnimSharingRed.AnimSharingRed"))

(event EventOnCharacterPossessed
  (|CallParentFunction)
  (Collision|SetCollisionResponsetoChannel (Variables|Default|GetCapsuleComponent) "ECC_Pawn" "ECR_Block")
  (for _array_element (Variables|/Game/BPs/Characters/Thermite/BP_ThermiteNest.BP_ThermiteNest_C|GetFollowingThermites (Variables|Default|GetNest))
    (AI|Components|Blackboard|SetValueasObject (AI|GetBlackboard (AI|GetAIController _array_element)) (Utilities|Name|MakeLiteralName "TargetActor") 0)))

(fn ConstructionScript
  (|CallParentFunction))