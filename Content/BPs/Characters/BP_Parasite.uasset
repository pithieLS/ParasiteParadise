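; BP_Parasite is the parasite character, a child Blueprint that exists as its own pawn while it is without a host.
; On death it calls OnParasiteDie on BP_ThirdPersonGameMode and prints a debug message that it died without a host.
; It passes possession events to its parent and destroys itself once unpossessed, so the actor does not persist after control leaves it.
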(event Collision|EventActorBeginOverlap
  (params (OtherActor :type Actor%20Object%20Reference)))

(event EventOnDie
  (Default|OnParasiteDie (.AsBP%20Third%20Person%20Game%20Mode (Utilities|Casting|CastToBP_ThirdPersonGameMode (Game|GetGameMode))))
  (Development|PrintString "parasite died without host"))

(event EventOnCharacterUnPossessed
  (|CallParentFunction)
  (Actor|DestroyActor))

(event EventOnCharacterPossessed
  (|CallParentFunction))

(fn ConstructionScript
  (|CallParentFunction))