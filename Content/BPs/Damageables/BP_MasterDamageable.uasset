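; Base damageable object Blueprint with health, a world-space healthbar widget and a destruction hook for subclasses.
; The Damages event subtracts health, updates the healthbar or, at zero, flags the object destroyed and calls the empty OnObjectDestruct event.
; Each hit also activates an optional Niagara damage effect.
; Tick rotates the healthbar to face the player camera until the object is destroyed.
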(event Custom|OnObjectDestruct)

(event EventBeginPlay
  (Variables|Default|SetHealth (Variables|Default|GetHealthMax))
  (bind _aswbp_damageable_healthbar (Utilities|Casting|CastToWBP_DamageableHealthbar (UserInterface|GetWidget (Variables|Default|GetHealthbar))))
  (Variables|Default|SetAs%20WBP%20Damageable%20Healthbar _aswbp_damageable_healthbar))

(event EventTick
  (params (DeltaSeconds :type Float%20%28single-precision%29))
  (if (not (Variables|Default|GetbIsDestroyed))
    (Transformation|SetWorldRotation (Variables|Default|GetHealthbar) (Math|Rotator|FindLookatRotation (Transformation|GetWorldLocation (Variables|Default|GetHealthbar)) (Camera|GetCameraLocation (Game|GetPlayerCameraManager 0))) false false)))

(event EventDamages
  (params (DamageAmount :type Integer) (HitComponent :type Actor%20Component%20Object%20Reference) (FromWho :type BP%20Master%20Character%20Object%20Reference))
  (bind _damageniagara (Variables|Default|GetDamageNiagara))
  (bind _output_get (Variables|Default|SetHealth (- (Variables|Default|GetHealth) DamageAmount)))
  (if (<= _output_get 0)
    (Variables|Default|SetbIsDestroyed true)
    (CallFunction|OnObjectDestruct)
    (else
      (Default|UpdateHealthbar (Variables|Default|GetAs%20WBP%20Damageable%20Healthbar) (Variables|Default|GetHealth) (Variables|Default|GetHealthMax))))
  (Utilities|IsValid _damageniagara
    (:Is%20Valid
      (Components|Activation|Activate _damageniagara true))))

(fn ConstructionScript)