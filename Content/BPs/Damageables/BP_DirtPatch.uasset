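; BP_DirtPatch is a damageable dirt patch that triggers the game's win when destroyed.
; It removes its inherited health bar on BeginPlay and responds only to damage from BP_Fox, forwarding it to the parent with a zero damage amount.
; On destruction it removes the dirt mesh, waits briefly, then calls OnWin on BP_ThirdPersonGameMode.
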(event EventBeginPlay
  (|CallParentFunction)
  (Components|DestroyComponent (Variables|Default|GetHealthbar)))

(event Collision|EventActorBeginOverlap
  (params (OtherActor :type Actor%20Object%20Reference)))

(event EventTick
  (params (DeltaSeconds :type Float%20%28single-precision%29)))

(event EventDamages
  (params (DamageAmount :type Integer) (HitComponent :type Actor%20Component%20Object%20Reference) (FromWho :type BP%20Master%20Character%20Object%20Reference))
  (Utilities|Casting|CastToBP_Fox FromWho)
  (|CallParentFunction 0 0 0))

(event EventOnObjectDestruct
  (bind _asbp_third_person_game_mode (Utilities|Casting|CastToBP_ThirdPersonGameMode (Game|GetGameMode)))
  (Components|DestroyComponent (Variables|Default|GetDirtPatchSM))
  (Utilities|FlowControl|Delay 2.0)
  (Default|OnWin _asbp_third_person_game_mode))

(fn ConstructionScript
  (|CallParentFunction))