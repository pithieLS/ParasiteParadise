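; BP_SwingingBoulder is a damageable boulder trap that is released when its support is destroyed and deals lethal-scale damage to the fox.
; On destruction, the geometry collection support simulates physics with a spawned FS_MasterField, and the support rope is removed.
; A looping timeline then swings the rope pivot between two rotations.
; The first overlap with BP_Fox applies damage, stops the swing and disables collision on child primitive components.
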(event OnComponentBeginOverlap(BoudlerCollider)
  (params (OverlappedComponent :type Primitive%20Component%20Object%20Reference) (OtherActor :type Actor%20Object%20Reference) (OtherComp :type Primitive%20Component%20Object%20Reference) (OtherBodyIndex :type Integer) (bFromSweep :type Boolean) (SweepResult :type Hit%20Result%20Structure%20%28by%20ref%29))
  (bind _asbp_fox (Utilities|Casting|CastToBP_Fox OtherActor))
  (Utilities|FlowControl|DoOnce false
    (:Completed
      (Class|BPIGlobalInteraction|ReceiveDamages(Message) _asbp_fox 999)
      (CallFunction|StopSwing)
      (for _array_element (Components|GetChildrenComponents (Variables|Default|GetDefaultSceneRoot) true)
        (bind _asprimitive_component (Utilities|Casting|CastToPrimitiveComponent _array_element))
        (Collision|SetCollisionEnabled _asprimitive_component "NoCollision")))))

(event Custom|StartSwing
  (bind _swingtrack (Timeline|Swing Play)
    (:Update
      (Transformation|SetRelativeRotation (Variables|Default|GetRopePivotPoint) (Math|Rotator|Lerp(Rotator) (Variables|Default|GetStartRotation) (Variables|Default|GetTargetRotation) _swingtrack) false false))
    (:Finished
      (Utilities|FlowControl|Delay 0.1)
      (Timeline|Swing PlayFromStart))))

(event Custom|StopSwing
  (bind _swingtrack (Timeline|Swing Stop)
    (:Update
      (Transformation|SetRelativeRotation (Variables|Default|GetRopePivotPoint) (Math|Rotator|Lerp(Rotator) (Variables|Default|GetStartRotation) (Variables|Default|GetTargetRotation) _swingtrack) false false))
    (:Finished
      (Utilities|FlowControl|Delay 0.1)
      (Timeline|Swing PlayFromStart))))

(event EventBeginPlay
  (|CallParentFunction))

(event EventTick
  (params (DeltaSeconds :type Float%20%28single-precision%29)))

(event EventOnObjectDestruct
  (bind _gc_support (Variables|Default|GetGC_Support))
  (Collision|SetCollisionResponsetoChannel _gc_support "ECC_Pawn" "ECR_Ignore")
  (Collision|SetCollisionResponsetoChannel _gc_support "ECC_Camera" "ECR_Ignore")
  (Collision|SetCollisionEnabled _gc_support "NoCollision")
  (Collision|SetCollisionEnabled _gc_support "QueryAndPhysics")
  (Physics|SetSimulatePhysics _gc_support true)
  (Game|SpawnActorfromClass "/Engine/EditorResources/FieldNodes/FS_MasterField.FS_MasterField_C" (Math|Transform|MakeTransform (Transformation|GetWorldLocation (Variables|Default|GetGC_Support)) "0, 0, 0" "1.000000,1.000000,1.000000") "Undefined" "MultiplyWithRoot" 0 0)
  (CallFunction|StartSwing)
  (Components|DestroyComponent (Variables|Default|GetSupportRope)))

(fn ConstructionScript
  (|CallParentFunction))