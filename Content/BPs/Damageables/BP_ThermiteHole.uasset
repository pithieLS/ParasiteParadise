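; BP_ThermiteHole is a damageable wooden pallet obstacle that only BP_Thermite actors can damage and break.
; When the player's thermite enters ThermitesZone, its nest's following thermites get the obstacle as AI prey and the healthbar shows; leaving reverses both.
; On destruction, the mesh is swapped for a Geometry Collection blown apart by a radial impulse, prey is cleared, and the actor is destroyed after a short delay.
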(event OnComponentBeginOverlap(ThermitesZone)
  (params (OverlappedComponent :type Primitive%20Component%20Object%20Reference) (OtherActor :type Actor%20Object%20Reference) (OtherComp :type Primitive%20Component%20Object%20Reference) (OtherBodyIndex :type Integer) (bFromSweep :type Boolean) (SweepResult :type Hit%20Result%20Structure%20%28by%20ref%29))
  (bind _healthbar (Variables|Default|GetHealthbar))
  (bind _asbp_thermite (Utilities|Casting|CastToBP_Thermite OtherActor))
  (if (Utilities|CheckifPlayerControlled _asbp_thermite)
    (Variables|Default|SetControlledThermite _asbp_thermite)
    (CallFunction|SetAllThermitesPrey _asbp_thermite self)
    (Utilities|IsValid _healthbar
      (:Is%20Valid
        (Rendering|SetVisibility _healthbar true false)))))

(event OnComponentEndOverlap(ThermitesZone)
  (params (OverlappedComponent :type Primitive%20Component%20Object%20Reference) (OtherActor :type Actor%20Object%20Reference) (OtherComp :type Primitive%20Component%20Object%20Reference) (OtherBodyIndex :type Integer))
  (bind _healthbar (Variables|Default|GetHealthbar))
  (bind _asbp_thermite (Utilities|Casting|CastToBP_Thermite OtherActor))
  (if (Utilities|CheckifPlayerControlled _asbp_thermite)
    (CallFunction|SetAllThermitesPrey _asbp_thermite)
    (Utilities|IsValid _healthbar
      (:Is%20Valid
        (Rendering|SetVisibility _healthbar false false)))))

(event EventOnObjectDestruct
  (bind _woodenpaletmesh (Variables|Default|GetWoodenPaletMesh))
  (Utilities|FlowControl|DoOnce false
    (:Completed
      (bind _returnvalue (AddComponent|AddGeometryCollectionComponent false (Transformation|GetRelativeTransform _woodenpaletmesh)))
      (Collision|SetCollisionResponsetoChannel _returnvalue "ECC_Camera" "ECR_Ignore")
      (Components|DestroyComponent _woodenpaletmesh)
      (Physics|AddRadialImpulse _returnvalue (Transformation|GetWorldLocation _returnvalue) 1e+02 5e+02 "RIF_Constant" false)
      (CallFunction|SetAllThermitesPrey (Variables|Default|GetControlledThermite))
      (Utilities|FlowControl|Delay 2.0)
      (Actor|DestroyActor))))

(event EventDamages
  (params (DamageAmount :type Integer) (HitComponent :type Actor%20Component%20Object%20Reference) (FromWho :type BP%20Master%20Character%20Object%20Reference))
  (Utilities|Casting|CastToBP_Thermite FromWho)
  (|CallParentFunction DamageAmount HitComponent FromWho))

(fn ConstructionScript)

(fn SetAllThermitesPrey
  (params (ControlledThermite :type BP%20Thermite%20Object%20Reference) (Prey :type Actor%20Object%20Reference))
  (for _array_element (Variables|/Game/BPs/Characters/Thermite/BP_ThermiteNest.BP_ThermiteNest_C|GetFollowingThermites (Variables|/Game/BPs/Characters/Thermite/BP_Thermite.BP_Thermite_C|GetNest ControlledThermite))
    (bind _asaic_thermite (Utilities|Casting|CastToAIC_Thermite (AI|GetAIController _array_element)))
    (Default|SetPrey _asaic_thermite Prey)))